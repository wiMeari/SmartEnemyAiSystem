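; Sword-wielding melee enemy built on a parent enemy class, with a combo attack, a leaping long-range attack and random blocking.
; Montage notifies time the sphere-trace damage to non-team members, the jump and sword spawn/removal; attacks are uninterruptible while playing.
; The leap launches along a suggested arc toward the target's velocity-predicted position and stops on landing.
; Blockable hits may trigger a timed block through the damage component before parent damage handling.
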(event `/Game/MyContent/Enemies/AI/BPI_EnemyAI.Attack`
  (params (AttackTarget :type "Actor Object Reference"))
  (`self.MeleeAttack` AttackTarget))

(event `MeleeAttack`
  (params (Target :type "Actor Object Reference"))
  (`parent.Attack` Target)
  (bind _notifyname (`|PlayMontage` (`self.Mesh`) "/Game/MyContent/Anim/Melee/AM_AS_Combo_Attack_02_01_Seq_Montage.AM_AS_Combo_Attack_02_01_Seq_Montage")
    (:`then`
      (set `/Game/MyContent/BP/DamageSys/BPC_DamageSystem.IsInterruptible` false (`self.BPC_DamageSystem`)))
    (:`OnCompleted`
      (`self.AttackEnd` Target :!label _label)
      (set `/Game/MyContent/BP/DamageSys/BPC_DamageSystem.IsInterruptible` true (`self.BPC_DamageSystem`)))
    (:`OnInterrupted`
      (goto _label))
    (:`OnNotifyBegin`
      (switch `name` _notifyname
        (:`Slash`
          (`self.SphereTraceDamage`))))))

(event `SphereTraceDamage`
  (bind _returnvalue (`self.K2_GetActorLocation`))
  ; 攻击辅助
  (bind (_outhits _returnvalue_2) (`KismetSystemLibrary.SphereTraceMultiForObjects` _returnvalue (+ _returnvalue (* (`self.GetActorForwardVector`) 200.0)) 0.0 (`|MakeArray` "ObjectTypeQuery3" :!type "EObjectTypeQuery Enum")))
  (if _returnvalue_2
    (`/Game/MyContent/BP/Attack/BPC_Attacks.DamageAllNonTeamMembers` (`self.BPC_Attacks`) _outhits (make `/Game/MyContent/BP/DamageSys/S_DamageInfo` 30.0 "NewEnumerator1"))))

(event `JumpToAttackTarget`
  (params (Actor :type "Actor Object Reference"))
  ; 攻击辅助
  (bind _location (`self.CalcFutureActorLocation` Actor))
  (bind _outlaunchvelocity (`GameplayStatics.SuggestProjectileVelocity_CustomArc` (`self.K2_GetActorLocation`) (`KismetMathLibrary.MakeVector` (.x _location) (.y _location) (+ (.z _location) 100.0))))
  (`self.LaunchCharacter` (* _outlaunchvelocity (`KismetMathLibrary.MakeVector` 2.0 2.0 1.0)) true true)
  (add `self.LandedDelegate` (delegate `LandedDelegate_事件`)))

(event `LonggRangeAttack`
  (params (Target :type "Actor Object Reference"))
  (`parent.Attack` Target)
  (bind _notifyname (`|PlayMontage` (`self.Mesh`) "/Game/MyContent/Anim/Melee/AM_JumpAttack.AM_JumpAttack")
    (:`then`
      (set `/Game/MyContent/BP/DamageSys/BPC_DamageSystem.IsInterruptible` false (`self.BPC_DamageSystem`)))
    (:`OnCompleted`
      (`self.AttackEnd` Target :!label _label_2)
      (set `/Game/MyContent/BP/DamageSys/BPC_DamageSystem.IsInterruptible` true (`self.BPC_DamageSystem`)))
    (:`OnInterrupted`
      (goto _label_2))
    (:`OnNotifyBegin`
      (switch `name` _notifyname
        (:`Slash`
          (`self.SphereTraceDamage`))
        (:`Jump`
          (`self.JumpToAttackTarget` Target))))))

(event `LandedDelegate_事件` :!signature `self.LandedDelegate`
  (params (Hit :type "HitResult Structure (by ref)"))
  ; 攻击辅助
  (remove `self.LandedDelegate` (delegate `LandedDelegate_事件`))
  (`MovementComponent.StopMovementImmediately` (`self.CharacterMovement`)))

(event `/Game/MyContent/Enemies/AI/BPI_EnemyAI.EquipWeapon`
  (bind _notifyname (`|PlayMontage` (`self.Mesh`) "/Game/MyContent/Anim/Melee/AM_Idle_to_Idle_Equip.AM_Idle_to_Idle_Equip")
    (:`OnCompleted`
      (`self.OnWeaponEquipped`))
    (:`OnNotifyBegin`
      (switch `name` _notifyname
        (:`WieldSword`
          (bind _returnvalue (`|SpawnActorFromClass` "/Game/MyContent/Weapon/BP_WeaponSword.BP_WeaponSword_C" (`KismetMathLibrary.MakeTransform` (0.0 0.0 0.0)) "AlwaysSpawn" "MultiplyWithRoot" null null))
          (bind _output_get (set `self.WeaponActor` _returnvalue))
          (`self.K2_AttachToComponent` _output_get (`self.Mesh`) "hand_r_SwardSocket" "KeepRelative" "KeepRelative" "KeepRelative" true)
          (set `self.IsWieldingWeapon` true))))))

(event `/Game/MyContent/Enemies/AI/BPI_EnemyAI.UnequipWeapon`
  (bind _notifyname (`|PlayMontage` (`self.Mesh`) "/Game/MyContent/Anim/Melee/AM_Idle_to_Idle_UnEquip_Montage.AM_Idle_to_Idle_UnEquip_Montage")
    (:`OnCompleted`
      (`self.OnWeaponUnequipped`))
    (:`OnNotifyBegin`
      (switch `name` _notifyname
        (:`DropSword`
          (`self.K2_DestroyActor` (`self.WeaponActor`))
          (set `self.IsWieldingWeapon` false))))))

(event `StartBlock`
  ; 敌人格挡
  (`KismetSystemLibrary.K2_ClearAndInvalidateTimerHandle` (`self.HoldBlockTimer`))
  (`MovementComponent.StopMovementImmediately` (`self.CharacterMovement`))
  (set `/Game/MyContent/BP/DamageSys/BPC_DamageSystem.IsBlocking` true (`self.BPC_DamageSystem`))
  (set `self.BlockState` "NewEnumerator1")
  (`MovementComponent.StopMovementImmediately` (`self.CharacterMovement`))
  (bind _returnvalue (`KismetSystemLibrary.K2_SetTimerDelegate` (`|CreateDelegate` :!event `EndBlock`) 2.0))
  (set `self.HoldBlockTimer` _returnvalue))

(event `self.BPC_DamageSystem.OnBlocked`
  (params (CanBeParried :type Boolean))
  ; 敌人格挡
  (set `self.BlockState` "NewEnumerator2")
  (`KismetSystemLibrary.K2_ClearAndInvalidateTimerHandle` (`self.HoldBlockTimer`))
  (`|PlayMontage` (`self.Mesh`) "/Game/MyContent/Anim/Melee/Block/AM_AS_Block_End_Seq.AM_AS_Block_End_Seq"
    (:`OnCompleted`
      _)
    (:`OnInterrupted`
      _))
  (`self.EndBlock`))

(event `EndBlock`
  ; 敌人格挡
  (set `/Game/MyContent/BP/DamageSys/BPC_DamageSystem.IsBlocking` false (`self.BPC_DamageSystem`))
  (set `self.BlockState` "NewEnumerator0")
  (`self.OnBlockEnd`))

(fn `CalcFutureActorLocation`
  (params (Actor :type "Actor Object Reference") (Time :type "Float (double-precision)" :default 1.0))
  (returns (Location :type "Vector Structure"))
  (return (+ (`self.K2_GetActorLocation` Actor) (* (* (`self.GetVelocity` Actor) (1.0 1.0 0.0)) Time))))

(fn `GetIdealRange`
  (returns (AttackRadius :type "Float (double-precision)") (DefendRadius :type "Float (double-precision)"))
  (return 200.0 400.0))

(fn `GetPatrolRoute`
  (returns (ReturnValue :type "/Game/MyContent/Enemies/AI/BP_PatrolRoute Object Reference"))
  (bind _returnvalue (`parent.GetPatrolRoute`))
  (return _returnvalue))

(fn `TakeDamage`
  (params (DamageInfo :type "/Game/MyContent/BP/DamageSys/S_DamageInfo Structure") (`Damage Source` :type "Actor Object Reference"))
  (returns (WasDamage :type Boolean))
  (if (`.CanBeBlock_16_6AD336DE49674E54E87352A7DBC718A6` (break `/Game/MyContent/BP/DamageSys/S_DamageInfo` DamageInfo))
    (`self.TryToBlock`))
  (bind _wasdamage (`parent.TakeDamage` DamageInfo `Damage Source`))
  (return _wasdamage))

(fn `TryToBlock`
  (if (<= (`KismetMathLibrary.RandomFloat`) (`self.Block Chance`))
    (`self.StartBlock`)))

(fn `UserConstructionScript`
  (`parent.UserConstructionScript`))