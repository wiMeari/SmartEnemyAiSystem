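; BP_EnemyMelee is a sword-wielding melee enemy that supplies attack, equip and unequip actions plus its ideal attack and defend ranges.
; Each action plays a montage, with notifies timing the forward sphere-trace damage and the sword's spawn, socket attachment and destruction.
; Attacking makes the damage system uninterruptible until the montage completes or is interrupted.
; Event dispatchers report attack end and completed weapon changes.
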(event `/Game/MyContent/Enemies/AI/BPI_EnemyAI.Attack`
  (bind _returnvalue (`self.K2_GetActorLocation`))
  (bind _notifyname (`|PlayMontage` (`self.Mesh`) "/Game/MyContent/Anim/Melee/AM_AS_Combo_Attack_02_01_Seq_Montage.AM_AS_Combo_Attack_02_01_Seq_Montage")
    (:`then`
      (set `/Game/MyContent/BP/DamageSys/BPC_DamageSystem.IsInterruptible` false (`self.BPC_DamageSystem`)))
    (:`OnCompleted`
      (`self.OnAttackEnd` :!label _label)
      (set `/Game/MyContent/BP/DamageSys/BPC_DamageSystem.IsInterruptible` true (`self.BPC_DamageSystem`)))
    (:`OnInterrupted`
      (goto _label))
    (:`OnNotifyBegin`
      (switch `name` _notifyname
        (:`Slash`
          (bind (_outhit _returnvalue_2) (`KismetSystemLibrary.SphereTraceSingleForObjects` :`Start` _returnvalue :`End` (+ _returnvalue (* (`self.GetActorForwardVector`) 200.0)) :`Radius` 20.0 :`ObjectTypes` (`|MakeArray` "ObjectTypeQuery3" :!type "EObjectTypeQuery Enum") :`DrawDebugType` "ForDuration"))
          (if _returnvalue_2
            (message `/Game/MyContent/BP/BPI_Damageable.TakeDamage` (`.HitActor` (`GameplayStatics.BreakHitResult` _outhit)) (make `/Game/MyContent/BP/DamageSys/S_DamageInfo` 25.0 "NewEnumerator1"))))))))

(event `/Game/MyContent/Enemies/AI/BPI_EnemyAI.EquipWeapon`
  (bind _notifyname (`|PlayMontage` (`self.Mesh`) "/Game/MyContent/Anim/Melee/AM_Idle_to_Idle_Equip.AM_Idle_to_Idle_Equip")
    (:`OnCompleted`
      (`self.OnWeaponEquipped`))
    (:`OnNotifyBegin`
      (switch `name` _notifyname
        (:`WieldSword`
          (bind _returnvalue (`|SpawnActorFromClass` "/Game/MyContent/Weapon/BP_WeaponSword.BP_WeaponSword_C" (`KismetMathLibrary.MakeTransform` (0.0 0.0 0.0)) "AlwaysSpawn" "MultiplyWithRoot" null null))
          (bind _output_get (set `self.WeaponActor` _returnvalue))
          (`self.K2_AttachToComponent` _output_get (`self.Mesh`) "hand_r_SwardSocket" "KeepRelative" "KeepRelative" "KeepRelative" true)
          (set `self.IsWieldingWeapon` true))))))

(event `/Game/MyContent/Enemies/AI/BPI_EnemyAI.UnequipWeapon`
  (bind _notifyname (`|PlayMontage` (`self.Mesh`) "/Game/MyContent/Anim/Melee/AM_Idle_to_Idle_UnEquip_Montage.AM_Idle_to_Idle_UnEquip_Montage")
    (:`OnCompleted`
      (`self.OnWeaponUnequipped`))
    (:`OnNotifyBegin`
      (switch `name` _notifyname
        (:`DropSword`
          (`self.K2_DestroyActor` (`self.WeaponActor`))
          (set `self.IsWieldingWeapon` false))))))

(fn `GetIdealRange`
  (returns (AttackRadius :type "Float (double-precision)") (DefendRadius :type "Float (double-precision)"))
  (return 150.0 350.0))

(fn `UserConstructionScript`
  (`parent.UserConstructionScript`))