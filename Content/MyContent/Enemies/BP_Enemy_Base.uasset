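; Base enemy character Blueprint that provides health, damage reactions, movement speeds and data such as patrol route and combat ranges.
; A damage system component handles health, damage and healing, with a health bar widget created on BeginPlay.
; Its death and damage events drive the AIC_EnemyBase controller: death ragdolls the mesh and stops AI logic.
; Hits halt movement and freeze the AI during a reaction montage, then resume attacking the last known target.
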(event `InitValue`
  (bind _asaic_enemy_base (cast `/Game/MyContent/Enemies/AI/AIC_EnemyBase` (`AIBlueprintHelperLibrary.GetAIController` self)))
  (set `self.AIC Enemy Base` _asaic_enemy_base))

(event `self.ReceiveBeginPlay`
  (bind _bpc_damagesystem (`self.BPC_DamageSystem`))
  (`self.InitValue`)
  (bind _returnvalue (`|CreateWidget` "/Game/MyContent/BP/DamageSys/WBP_HealthBar.WBP_HealthBar_C" null self))
  (`WidgetComponent.SetWidget` (`self.Widget`) _returnvalue)
  (add `/Game/MyContent/BP/DamageSys/BPC_DamageSystem.OnDeath` _bpc_damagesystem (`|CreateDelegate` :!event `Die`))
  (add `/Game/MyContent/BP/DamageSys/BPC_DamageSystem.OnDamageResponse` _bpc_damagesystem (`|CreateDelegate` :!event `DamageResponse`)))

(event `Die`
  (bind _mesh (`self.Mesh`))
  (`PrimitiveComponent.SetCollisionEnabled` _mesh "QueryAndPhysics")
  (`PrimitiveComponent.SetSimulatePhysics` _mesh true)
  (`PrimitiveComponent.SetCollisionEnabled` (`self.CapsuleComponent`) "NoCollision")
  (bind _aic_enemy_base (`self.AIC Enemy Base`)
    (:`then`
      (`BrainComponent.StopLogic` (`AIController.BrainComponent` _aic_enemy_base) "")
      (`/Game/MyContent/Enemies/AI/AIC_EnemyBase.SetStateAsDead` _aic_enemy_base))
    (:`else`)))

(event `DamageResponse`
  (params (DamageResponse :type "/Game/MyContent/BP/DamageSys/E_DamageResponse Enum" :default "NewEnumerator0"))
  (`MovementComponent.StopMovementImmediately` (`self.CharacterMovement`))
  (`/Game/MyContent/Enemies/AI/AIC_EnemyBase.SetStateAsFrozen` (`self.AIC Enemy Base`))
  (`|PlayMontage` (`self.Mesh`) (`self.HitReactionMontage`)
    (:`OnCompleted`
      _)
    (:`OnInterrupted`
      _))
  (bind _aic_enemy_base (`self.AIC Enemy Base`)
    (:`then`
      (`/Game/MyContent/Enemies/AI/AIC_EnemyBase.SetStateAsAttack` _aic_enemy_base null true))
    (:`else`)))

(fn `GetCurrentHealth`
  (returns (Health :type "Float (double-precision)"))
  (return (`/Game/MyContent/BP/DamageSys/BPC_DamageSystem.Health` (`self.BPC_DamageSystem`))))

(fn `GetIdealRange`
  (returns (AttackRadius :type "Float (double-precision)") (DefendRadius :type "Float (double-precision)"))
  (return 150.0 350.0))

(fn `GetMaxHealth`
  (returns (Health :type "Float (double-precision)"))
  (return (`/Game/MyContent/BP/DamageSys/BPC_DamageSystem.MaxHealth` (`self.BPC_DamageSystem`))))

(fn `GetPatrolRoute`
  (returns (ReturnValue :type "/Game/MyContent/Enemies/AI/BP_PatrolRoute Object Reference"))
  (return (`self.PatrolRoute`)))

(fn `Heal`
  (params (HealthAmount :type "Float (double-precision)"))
  (returns (NewHealth :type "Float (double-precision)"))
  (bind _newhealth (`/Game/MyContent/BP/DamageSys/BPC_DamageSystem.Heal` (`self.BPC_DamageSystem`) HealthAmount))
  (return _newhealth))

(fn `IsAttacking`
  (returns (IsAttacking :type Boolean))
  (return (`self.IsAttackingState`)))

(fn `IsDead`
  (returns (Dead :type Boolean))
  (return (`/Game/MyContent/BP/DamageSys/BPC_DamageSystem.IsDead` (`self.BPC_DamageSystem`))))

(fn `SetMovementSpeed`
  (params (Speed :type "/Game/MyContent/Enemies/AI/Data/Enum/E_MovementSpeed Enum" :default "NewEnumerator0"))
  (returns (ReturnValue :type "Float (double-precision)"))
  (bind _output_get (set `CharacterMovementComponent.MaxWalkSpeed` (select `/Game/MyContent/Enemies/AI/Data/Enum/E_MovementSpeed` Speed :`NewEnumerator1` 200.0 :`NewEnumerator2` 300.0 :`NewEnumerator3` 500.0 :!type "Float (single-precision)") (`self.CharacterMovement`)))
  (return _output_get))

(fn `TakeDamage`
  (params (DamageInfo :type "/Game/MyContent/BP/DamageSys/S_DamageInfo Structure"))
  (returns (WasDamage :type Boolean))
  (bind _wasdamaged (`/Game/MyContent/BP/DamageSys/BPC_DamageSystem.TakeDamage` (`self.BPC_DamageSystem`) DamageInfo))
  (return _wasdamaged))

(fn `UserConstructionScript`
  (bind _bpc_damagesystem (`self.BPC_DamageSystem`))
  (set `/Game/MyContent/BP/DamageSys/BPC_DamageSystem.Health` 100.0 _bpc_damagesystem)
  (set `/Game/MyContent/BP/DamageSys/BPC_DamageSystem.MaxHealth` 100.0 _bpc_damagesystem))