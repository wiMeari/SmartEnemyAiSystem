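; BP_EnemyRanged is a rifle-wielding enemy character that extends a parent enemy class with ranged attack behavior.
; On BeginPlay it spawns a rifle and attaches it to the hand socket.
; Attack plays a firing montage, whose Fire notify shoots through BPCAttacks from the rifle toward the AI controller's target with blockable damage.
; It also supplies its ideal attack and defend ranges and maps movement states to walk speeds.
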(event `self.ReceiveBeginPlay`
  (`parent.ReceiveBeginPlay`)
  (`self.EquipWeapon`))

(event `/Game/MyContent/Enemies/AI/BPI_EnemyAI.EquipWeapon`
  (bind _returnvalue (`|SpawnActorFromClass` "/Game/MyContent/Weapon/BP_WeaponRifle.BP_WeaponRifle_C" (`KismetMathLibrary.MakeTransform` (0.0 0.0 0.0)) "Undefined" "MultiplyWithRoot" null null))
  (bind _output_get (set `self.WeaponActor` _returnvalue))
  (`self.K2_AttachToComponent` _output_get (`self.Mesh`) "hand_r_RifleSocket" "KeepRelative" "KeepRelative" "KeepRelative" true)
  (set `self.IsWieldingWeapon` true)
  (`self.OnWeaponEquipped`))

(event `/Game/MyContent/Enemies/AI/BPI_EnemyAI.UnequipWeapon`)

(event `/Game/MyContent/Enemies/AI/BPI_EnemyAI.Attack`
  (set `self.IsAttackingState` true)
  (bind _notifyname (`|PlayMontage` (`self.Mesh`) "/Game/MyContent/Anim/Rifle/AM/AM_FiringRifle_UE.AM_FiringRifle_UE")
    (:`OnCompleted`
      (`self.OnAttackEnd` :!label _label)
      (set `self.IsAttackingState` false))
    (:`OnInterrupted`
      (goto _label))
    (:`OnNotifyBegin`
      (switch `name` _notifyname
        (:`Fire`
          (bind _asaic_enemy_base (cast `/Game/MyContent/Enemies/AI/AIC_EnemyBase` (`AIBlueprintHelperLibrary.GetAIController` self)))
          (bind _attacktarget (`/Game/MyContent/Enemies/AI/AIC_EnemyBase.AttackTarget` _asaic_enemy_base)
            (:`then`
              (`/Game/MyContent/BP/Attack/BPC_Attacks.FireBullet` (`self.BPC_Attacks`) (`self.K2_GetActorLocation` (`self.WeaponActor`)) (`self.K2_GetActorLocation` _attacktarget) (make `/Game/MyContent/BP/DamageSys/S_DamageInfo` 20.0 "NewEnumerator2" "NewEnumerator0" false true)))
            (:`else`)))))))

(fn `GetIdealRange`
  (returns (AttackRadius :type "Float (double-precision)") (DefendRadius :type "Float (double-precision)"))
  (return 600.0 600.0))

(fn `SetMovementSpeed`
  (params (Speed :type "/Game/MyContent/Enemies/AI/Data/Enum/E_MovementSpeed Enum" :default "NewEnumerator0"))
  (returns (ReturnValue :type "Float (double-precision)"))
  (bind _output_get (set `CharacterMovementComponent.MaxWalkSpeed` (select `/Game/MyContent/Enemies/AI/Data/Enum/E_MovementSpeed` Speed :`NewEnumerator1` 250.0 :`NewEnumerator2` 300.0 :`NewEnumerator3` 500.0 :!type "Float (single-precision)") (`self.CharacterMovement`)))
  (return _output_get))

(fn `UserConstructionScript`
  (`parent.UserConstructionScript`))