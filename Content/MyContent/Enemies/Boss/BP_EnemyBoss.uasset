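; Boss enemy character, derived from a parent enemy, that fights with an axe, teleports and has an invincible floating phase.
; Attacks run through BPCAttacks or montage notifies, covering melee combos, jump attack, ground smash, thrown axe and AOE strike.
; Teleport is a fast, invisible AI flight with Niagara effects, while floating rides a spawned platform.
; Dispatchers report equip, teleport and float completion, and TakeDamage refreshes the boss health bar from BPCDamageSystem.
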(event `self.ReceiveBeginPlay`
  (bind _bpc_damagesystem (`self.BPC_DamageSystem`))
  (`parent.ReceiveBeginPlay`)
  (`WidgetComponent.SetWidget` (`self.Widget`) null)
  (bind _returnvalue (`|CreateWidget` "/Game/MyContent/HUD/WBP/WBP_BossHealth.WBP_BossHealth_C"))
  (bind _output_get (set `self.BossHealthBarWidget` _returnvalue))
  (`/Game/MyContent/HUD/WBP/WBP_BossHealth.UpdateHealthPercentage` _output_get (`/Game/MyContent/BP/DamageSys/BPC_DamageSystem.Health` _bpc_damagesystem) (`/Game/MyContent/BP/DamageSys/BPC_DamageSystem.MaxHealth` _bpc_damagesystem)))

(event `Teleport`
  (params (Location :type "Vector Structure") (Target :type "Actor Object Reference"))
  (bind _charactermovement (`self.CharacterMovement`))
  (if (`self.IsTeleport`)
    (`KismetSystemLibrary.DelayUntilNextTick`)
    (`self.OnTeleportEnd`)
    (else
      (set `self.IsTeleport` true)
      (`CharacterMovementComponent.SetMovementMode` _charactermovement "MOVE_Flying" 0)
      (set `CharacterMovementComponent.MaxFlySpeed` 5000.0 _charactermovement)
      (set `CharacterMovementComponent.MaxAcceleration` 99999.0 _charactermovement)
      (`SceneComponent.SetVisibility` (`self.Mesh`) false true)
      (`PrimitiveComponent.SetCollisionResponseToChannel` (`self.CapsuleComponent`) "ECC_Pawn" "ECR_Ignore")
      (bind _returnvalue (`NiagaraFunctionLibrary.SpawnSystemAtLocation` "/Game/MyContent/Particle/NS_FireBallDead.NS_FireBallDead" (`SceneComponent.GetSocketLocation` (`self.Mesh`) "spine_01")))
      (set `self.TeleportBodyEffect` _returnvalue)
      (bind _returnvalue_2 (`NiagaraFunctionLibrary.SpawnSystemAttached` "/Game/MyContent/Particle/NS_FireBall.NS_FireBall" (`self.Mesh`) "spine_01" (0.0 0.0 0.0) (struct) "KeepRelativeOffset"))
      (set `self.TeleportTrailEffect` _returnvalue_2)
      (`self.StopAnimMontage` null)
      (`|AIMoveTo` self Location Target 150.0
        (:`OnSuccess`
          _)
        (:`OnFail`
          _))
      (`self.TeleportEnd`))))

(event `TeleportEnd`
  (bind _charactermovement (`self.CharacterMovement`))
  (`MovementComponent.StopMovementImmediately` _charactermovement)
  (`CharacterMovementComponent.SetMovementMode` _charactermovement "MOVE_Walking" 0)
  (set `CharacterMovementComponent.MaxAcceleration` 1500.0 _charactermovement)
  (`SceneComponent.SetVisibility` (`self.Mesh`) true true)
  (`PrimitiveComponent.SetCollisionResponseToChannel` (`self.CapsuleComponent`) "ECC_Pawn" "ECR_Block")
  (`self.OnTeleportEnd`)
  (`KismetSystemLibrary.Delay` 0.5)
  (set `self.IsTeleport` false)
  (`|ExecutionSequence`
    (:`then_0`
      (bind _teleportbodyeffect (`self.TeleportBodyEffect`)
        (:`then`
          (`ActorComponent.Deactivate` _teleportbodyeffect)
          (add `NiagaraComponent.OnSystemFinished` _teleportbodyeffect (delegate `OnSystemFinished_事件`)))
        (:`else`)))
    (:`then_1`
      (bind _teleporttraileffect (`self.TeleportTrailEffect`)
        (:`then`
          (`ActorComponent.Deactivate` _teleporttraileffect)
          (add `NiagaraComponent.OnSystemFinished` _teleporttraileffect (delegate `OnSystemFinished_事件_0`)))
        (:`else`)))))

(event `OnSystemFinished_事件`
  (params (PSystem :type "NiagaraComponent Object Reference"))
  (`ActorComponent.K2_DestroyComponent` PSystem))

(event `/Game/MyContent/Enemies/AI/BPI_EnemyAI.EquipWeapon`
  (bind _returnvalue (`|SpawnActorFromClass` "/Game/MyContent/Weapon/BP_WeaponAxe.BP_WeaponAxe_C" (`KismetMathLibrary.MakeTransform` (0.0 0.0 0.0)) "Undefined" "MultiplyWithRoot" null null))
  (bind _output_get (set `self.WeaponActor` _returnvalue))
  (`self.K2_AttachToComponent` _output_get (`self.Mesh`) "hand_rAxeSocket" "KeepRelative" "KeepRelative" "KeepRelative" true)
  (set `self.IsWieldingWeapon` true)
  (`KismetSystemLibrary.DelayUntilNextTick`)
  (`self.OnWeaponEquipped`))

(event `OnSystemFinished_事件_0`
  (params (PSystem :type "NiagaraComponent Object Reference"))
  (`ActorComponent.K2_DestroyComponent` PSystem))

(event `/Game/MyContent/Enemies/AI/BPI_EnemyAI.UnequipWeapon`
  (`self.K2_DestroyActor` (`self.WeaponActor`))
  (set `self.IsWieldingWeapon` false)
  (`KismetSystemLibrary.DelayUntilNextTick`)
  (`self.OnWeaponUnequipped`))

(event `AttackCombo1`
  (params (Target :type "Actor Object Reference"))
  (`/Game/MyContent/BP/Attack/BPC_Attacks.MeleeAttack` (`self.BPC_Attacks`) (make `/Game/MyContent/BP/Attack/S_AttackInfo` Target "/Game/MyContent/Anim/Axe/AM_Axe_Combo1.AM_Axe_Combo1" (make `/Game/MyContent/BP/DamageSys/S_DamageInfo` 30.0 "NewEnumerator1" "NewEnumerator0" false true true)) 40.0 250.0))

(event `AttackCombo2`
  (params (Target :type "Actor Object Reference"))
  (`self.Attack` Target)
  (bind _notifyname (`|PlayMontage` (`self.Mesh`) "/Game/MyContent/Anim/Axe/AM_AxeCombo2.AM_AxeCombo2")
    (:`OnCompleted`
      (`self.AttackEnd` Target :!label _label))
    (:`OnInterrupted`
      (goto _label))
    (:`OnNotifyBegin`
      (switch `name` _notifyname
        (:`Slash`
          (`/Game/MyContent/BP/Attack/BPC_Attacks.SphereTraceDamage` (`self.BPC_Attacks`) (make `/Game/MyContent/BP/DamageSys/S_DamageInfo` 30.0 "NewEnumerator1" "NewEnumerator0" false true true) 40.0 250.0))
        (:`AOESlash`
          (`/Game/MyContent/BP/Attack/BPC_Attacks.AOEDamage` (`self.BPC_Attacks`) null 250.0 (make `/Game/MyContent/BP/DamageSys/S_DamageInfo` 35.0 "NewEnumerator3" "NewEnumerator0" false false false true)))))))

(event `ThrowAxe`
  (params (target :type "Actor Object Reference"))
  (`/Game/MyContent/Enemies/AI/BPI_EnemyAI.Attack` target)
  (bind _notifyname (`|PlayMontage` (`self.Mesh`) "/Game/MyContent/Anim/Axe/AM_AxeThorw.AM_AxeThorw")
    (:`OnCompleted`
      (`SceneComponent.SetVisibility` (`/Game/MyContent/Weapon/BP_WeaponBase.Nodachi_Sword` (`self.WeaponActor`)) true false :!label _label_2)
      (`self.AttackEnd` target))
    (:`OnInterrupted`
      (goto _label_2))
    (:`OnNotifyBegin`
      (switch `name` _notifyname
        (:`Throw`
          (`SceneComponent.SetVisibility` (`/Game/MyContent/Weapon/BP_WeaponBase.Nodachi_Sword` (`self.WeaponActor`)) false false)
          (bind _returnvalue (`|SpawnActorFromClass` "/Game/MyContent/BP/Projectile/BP_Axe.BP_Axe_C" (`KismetMathLibrary.MakeTransform` (`SceneComponent.GetSocketLocation` (`self.Mesh`) "hand_rAxeSocket") (`KismetMathLibrary.FindLookAtRotation` (`self.K2_GetActorLocation`) (`self.K2_GetActorLocation` target))) "Undefined" "MultiplyWithRoot" null 4000.0 4000.0 0.0 self))
          (`PrimitiveComponent.IgnoreActorWhenMoving` (`/Game/MyContent/BP/Projectile/BP_ProjectileBase.Sphere` _returnvalue) self true)
          (add `/Game/MyContent/BP/Projectile/BP_ProjectileBase.OnProjectileImpact` _returnvalue (delegate `OnProjectileImpact_事件`)))))))

(event `OnProjectileImpact_事件`
  (params (OtherActor :type "Actor Object Reference") (Hit :type "HitResult Structure"))
  (message `/Game/MyContent/BP/DamageSys/BPI_Damageable.TakeDamage` OtherActor (make `/Game/MyContent/BP/DamageSys/S_DamageInfo` 30.0 "NewEnumerator2" "NewEnumerator0" false true) self)
  (`self.K2_DestroyActor` (stale `ThrowAxe` _returnvalue)))

(event `QuickAttack`
  (params (Target :type "Actor Object Reference"))
  (`/Game/MyContent/BP/Attack/BPC_Attacks.MeleeAttack` (`self.BPC_Attacks`) (make `/Game/MyContent/BP/Attack/S_AttackInfo` Target "/Game/MyContent/Anim/Axe/AM_AxeQuickAttack.AM_AxeQuickAttack" (make `/Game/MyContent/BP/DamageSys/S_DamageInfo` 30.0 "NewEnumerator1" "NewEnumerator0" false true true)) 40.0 250.0))

(event `StartFloat`
  (bind _returnvalue (`self.K2_GetActorLocation`))
  (set `/Game/MyContent/BP/DamageSys/BPC_DamageSystem.IsInvincible` true (`self.BPC_DamageSystem`))
  (bind _outhit (`KismetSystemLibrary.LineTraceSingle` _returnvalue (* _returnvalue (1.0 1.0 -1000.0)) "TraceTypeQuery1"))
  (bind _returnvalue_2 (`|SpawnActorFromClass` "/Game/MyContent/Enemies/Boss/BP_FloatingPlatform.BP_FloatingPlatform_C" (`KismetMathLibrary.MakeTransform` (`.Location` (`GameplayStatics.BreakHitResult` _outhit))) "Undefined" "MultiplyWithRoot" null null))
  (bind _output_get (set `self.FloatingPlatform` _returnvalue_2))
  (add `/Game/MyContent/Enemies/Boss/BP_FloatingPlatform.FloatTimelineFinished` _output_get (delegate `FloatTimelineFinished_事件`)))

(event `FloatTimelineFinished_事件`
  (remove `/Game/MyContent/Enemies/Boss/BP_FloatingPlatform.FloatTimelineFinished` (stale `StartFloat` _output_get) (delegate `FloatTimelineFinished_事件`))
  (`self.OnFloatingHeightReached`))

(event `StopFloat`
  (bind _floatingplatform (`self.FloatingPlatform`)
    (:`then`
      (`/Game/MyContent/Enemies/Boss/BP_FloatingPlatform.StopFloating` _floatingplatform)
      (add `/Game/MyContent/Enemies/Boss/BP_FloatingPlatform.FloatTimelineFinished` _floatingplatform (delegate `FloatTimelineFinished_事件_0`)))
    (:`else`
      (`KismetSystemLibrary.DelayUntilNextTick`)
      (set `/Game/MyContent/BP/DamageSys/BPC_DamageSystem.IsInvincible` false (`self.BPC_DamageSystem`) :!label _label_3)
      (`self.OnFloatingHeightReached`)
      (`self.K2_DestroyActor` _floatingplatform)
      (`self.OnFloatingEnded`))))

(event `JumpAttack`
  (params (AttackTarget :type "Actor Object Reference"))
  (`/Game/MyContent/BP/Attack/BPC_Attacks.LongRangeMeleeAttack` (`self.BPC_Attacks`) (make `/Game/MyContent/BP/Attack/S_AttackInfo` AttackTarget "/Game/MyContent/Anim/Axe/AM_AxeJumpAttack.AM_AxeJumpAttack" (make `/Game/MyContent/BP/DamageSys/S_DamageInfo` 0.0 "NewEnumerator3" "NewEnumerator0" false false false true))))

(event `FloatTimelineFinished_事件_0`
  (remove `/Game/MyContent/Enemies/Boss/BP_FloatingPlatform.FloatTimelineFinished` (stale `StopFloat` _floatingplatform) (delegate `FloatTimelineFinished_事件_0`))
  (goto _label_3))

(event `GroundSmash`
  (params (Target :type "Actor Object Reference"))
  (`/Game/MyContent/BP/Attack/BPC_Attacks.GroundSmash` (`self.BPC_Attacks`) (make `/Game/MyContent/BP/Attack/S_AttackInfo` Target "/Game/MyContent/Anim/Melee/AM_MeleeGroundSmash.AM_MeleeGroundSmash" (make `/Game/MyContent/BP/DamageSys/S_DamageInfo` 40.0 "NewEnumerator3" "NewEnumerator1")) 650.0))

(event `AOETrail`
  (params (Target :type "Actor Object Reference"))
  (`self.Attack` Target)
  (bind _notifyname (`|PlayMontage` (`self.Mesh`) "/Game/MyContent/Anim/Axe/AM_AxeBattlecry.AM_AxeBattlecry")
    (:`OnCompleted`
      (`self.AttackEnd` Target))
    (:`OnNotifyBegin`
      (switch `name` _notifyname
        (:`Strike`
          (bind _returnvalue (`|SpawnActorFromClass` "/Game/MyContent/BP/AOE/BP_AOEBase.BP_AOEBase_C" (`KismetMathLibrary.MakeTransform` (`self.K2_GetActorLocation` Target)) "Undefined" "MultiplyWithRoot" null false true false null))
          (add `/Game/MyContent/BP/AOE/BP_AOEBase.OnAOEOverlapActor` _returnvalue (delegate `OnAOEOverlapActor_事件`))
          (`/Game/MyContent/BP/AOE/BP_AOEBase.Trigger` _returnvalue))))))

(event `OnAOEOverlapActor_事件`
  (params (Actor :type "Actor Object Reference"))
  (bind _teamnum (message `/Game/MyContent/BP/DamageSys/BPI_Damageable.GetTeamNum` Actor))
  (if (!= _teamnum (`self.TeamNum`))
    (message `/Game/MyContent/BP/DamageSys/BPI_Damageable.TakeDamage` Actor (make `/Game/MyContent/BP/DamageSys/S_DamageInfo` 40.0 "NewEnumerator3") self)))

(fn `SetMovementSpeed`
  (params (Speed :type "/Game/MyContent/Enemies/AI/Data/Enum/E_MovementSpeed Enum" :default "NewEnumerator0"))
  (returns (ReturnValue :type "Float (double-precision)"))
  (bind _output_get (set `CharacterMovementComponent.MaxWalkSpeed` (select `/Game/MyContent/Enemies/AI/Data/Enum/E_MovementSpeed` Speed :`NewEnumerator1` 100.0 :`NewEnumerator2` 200.0 :`NewEnumerator3` 350.0 :!type "Float (single-precision)") (`self.CharacterMovement`)))
  (return _output_get))

(fn `TakeDamage`
  (params (DamageInfo :type "/Game/MyContent/BP/DamageSys/S_DamageInfo Structure") (`Damage Source` :type "Actor Object Reference"))
  (returns (WasDamage :type Boolean))
  (bind _bpc_damagesystem (`self.BPC_DamageSystem`))
  (bind _wasdamage (`parent.TakeDamage` DamageInfo `Damage Source`))
  (`/Game/MyContent/HUD/WBP/WBP_BossHealth.UpdateHealthPercentage` (`self.BossHealthBarWidget`) (`/Game/MyContent/BP/DamageSys/BPC_DamageSystem.Health` _bpc_damagesystem) (`/Game/MyContent/BP/DamageSys/BPC_DamageSystem.MaxHealth` _bpc_damagesystem))
  (return _wasdamage))

(fn `UserConstructionScript`
  (bind _bpc_damagesystem (`self.BPC_DamageSystem`))
  (`parent.UserConstructionScript`)
  (bind _output_get (set `/Game/MyContent/BP/DamageSys/BPC_DamageSystem.MaxHealth` 500.0 _bpc_damagesystem))
  (set `/Game/MyContent/BP/DamageSys/BPC_DamageSystem.Health` _output_get _bpc_damagesystem))