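; Mage enemy character with ground smash, basic magic and barrage attacks, a teleport and a self-heal, plus its own movement speeds and ideal ranges.
; Attack events pass montage and damage info to BPCAttacks.
; Teleport fakes a blink by AI-moving the hidden, fast-flying mage through pawns with Niagara effects.
; Healing spawns a ground-traced AOE that heals only the mage by max-health percentage, with dispatchers signaling when teleport and heal end.
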(event `GroundSmashAttack`
  (params (AttackTarget :type "Actor Object Reference"))
  ; 攻击
  (`/Game/MyContent/BP/Attack/BPC_Attacks.GroundSmash` (`self.BPC_Attacks`) (make `/Game/MyContent/BP/Attack/S_AttackInfo` AttackTarget "/Game/MyContent/Anim/Magic/AM_MageGroundSmash.AM_MageGroundSmash" (make `/Game/MyContent/BP/DamageSys/S_DamageInfo` 25.0 "NewEnumerator3")) 300.0))

(event `BasicAttack`
  (params (Target :type "Actor Object Reference"))
  ; 攻击
  (`/Game/MyContent/BP/Attack/BPC_Attacks.MageBasicAttack` (`self.BPC_Attacks`) (make `/Game/MyContent/BP/Attack/S_AttackInfo` Target "/Game/MyContent/Anim/Magic/AM_Magic_Standing1HMagicAttack01_UE.AM_Magic_Standing1HMagicAttack01_UE" (make `/Game/MyContent/BP/DamageSys/S_DamageInfo` 30.0 "NewEnumerator2"))))

(event `BarrageAttack`
  (params (Target :type "Actor Object Reference"))
  ; 攻击
  (`/Game/MyContent/BP/Attack/BPC_Attacks.MageBarrageAttack` (`self.BPC_Attacks`) (make `/Game/MyContent/BP/Attack/S_AttackInfo` Target "/Game/MyContent/Anim/Magic/AM_MageHitReaction.AM_MageHitReaction" (make `/Game/MyContent/BP/DamageSys/S_DamageInfo` 15.0 "NewEnumerator2"))))

(event `Teleport`
  (params (Location :type "Vector Structure"))
  (bind _charactermovement (`self.CharacterMovement`))
  (if (`self.IsTeleport`)
    (`KismetSystemLibrary.DelayUntilNextTick`)
    (`self.OnTeleportEnd`)
    (else
      (set `self.IsTeleport` true)
      (`CharacterMovementComponent.SetMovementMode` _charactermovement "MOVE_Flying" 0)
      (set `CharacterMovementComponent.MaxFlySpeed` 5000.0 _charactermovement)
      (set `CharacterMovementComponent.MaxAcceleration` 99999.0 _charactermovement)
      (`SceneComponent.SetVisibility` (`self.Mesh`) false true)
      (`PrimitiveComponent.SetCollisionResponseToChannel` (`self.CapsuleComponent`) "ECC_Pawn" "ECR_Ignore")
      (bind _returnvalue (`NiagaraFunctionLibrary.SpawnSystemAtLocation` "/Game/MyContent/Particle/NS_FireBallDead.NS_FireBallDead" (`SceneComponent.GetSocketLocation` (`self.Mesh`) "spine_01")))
      (set `self.TeleportBodyEffect` _returnvalue)
      (bind _returnvalue_2 (`NiagaraFunctionLibrary.SpawnSystemAttached` "/Game/MyContent/Particle/NS_FireBall.NS_FireBall" (`self.Mesh`) "spine_01" (0.0 0.0 0.0) (struct) "KeepRelativeOffset"))
      (set `self.TeleportTrailEffect` _returnvalue_2)
      (`self.StopAnimMontage` null)
      (`|AIMoveTo` self Location null 15.0
        (:`OnSuccess`
          _)
        (:`OnFail`
          _))
      (`self.TeleportEnd`))))

(event `TeleportEnd`
  (bind _charactermovement (`self.CharacterMovement`))
  (`MovementComponent.StopMovementImmediately` _charactermovement)
  (`CharacterMovementComponent.SetMovementMode` _charactermovement "MOVE_Walking" 0)
  (set `CharacterMovementComponent.MaxAcceleration` 1500.0 _charactermovement)
  (`SceneComponent.SetVisibility` (`self.Mesh`) true true)
  (`PrimitiveComponent.SetCollisionResponseToChannel` (`self.CapsuleComponent`) "ECC_Pawn" "ECR_Block")
  (`self.OnTeleportEnd`)
  (`KismetSystemLibrary.Delay` 0.5)
  (set `self.IsTeleport` false)
  (`|ExecutionSequence`
    (:`then_0`
      (bind _teleportbodyeffect (`self.TeleportBodyEffect`)
        (:`then`
          (`ActorComponent.Deactivate` _teleportbodyeffect)
          (add `NiagaraComponent.OnSystemFinished` _teleportbodyeffect (delegate `OnSystemFinished_事件`)))
        (:`else`)))
    (:`then_1`
      (bind _teleporttraileffect (`self.TeleportTrailEffect`)
        (:`then`
          (`ActorComponent.Deactivate` _teleporttraileffect)
          (add `NiagaraComponent.OnSystemFinished` _teleporttraileffect (delegate `OnSystemFinished_事件_0`)))
        (:`else`)))))

(event `OnSystemFinished_事件`
  (params (PSystem :type "NiagaraComponent Object Reference"))
  (`ActorComponent.K2_DestroyComponent` PSystem))

(event `OnSystemFinished_事件_0`
  (params (PSystem :type "NiagaraComponent Object Reference"))
  (`ActorComponent.K2_DestroyComponent` PSystem))

(event `HealOverTime`
  (bind _returnvalue (`self.K2_GetActorLocation`))
  (`|PlayMontage` (`self.Mesh`) "/Game/MyContent/Anim/Magic/AM_MagicHeal.AM_MagicHeal"
    (:`then`
      (bind (_outhit _returnvalue_2) (`KismetSystemLibrary.LineTraceSingle` _returnvalue (* _returnvalue (0.0 0.0 -1000.0)) "TraceTypeQuery1"))
      (if _returnvalue_2
        (bind _returnvalue_3 (`|SpawnActorFromClass` "/Game/MyContent/BP/AOE/BP_AOE_Heal.BP_AOE_Heal_C" (`KismetMathLibrary.MakeTransform` (`.Location` (`GameplayStatics.BreakHitResult` _outhit))) "Undefined" "MultiplyWithRoot" null 1.0 10.0 false true true null))
        (bind _output_get (set `self.HealAOE` _returnvalue_3))
        (add `/Game/MyContent/BP/AOE/BP_AOEBase.OnAOEOverlapActor` _output_get (delegate `OnAOEOverlapActor_事件`))
        (else
          (`self.StopAnimMontage` null))))
    (:`OnCompleted`
      (`self.HealOverTimeEnded` :!label _label))
    (:`OnInterrupted`
      (goto _label))))

(event `OnAOEOverlapActor_事件`
  (params (Actor :type "Actor Object Reference"))
  (if (== Actor self)
    (`/Game/MyContent/BP/DamageSys/BPI_Damageable.Heal` (* 0.05 (`/Game/MyContent/BP/DamageSys/BPC_DamageSystem.MaxHealth` (`self.BPC_DamageSystem`))))))

(event `HealOverTimeEnded`
  (`self.OnHealOverTimeEnd`)
  (bind _healaoe (`self.HealAOE`)
    (:`then`
      (`self.K2_DestroyActor` _healaoe))
    (:`else`)))

(fn `GetIdealRange`
  (returns (AttackRadius :type "Float (double-precision)") (DefendRadius :type "Float (double-precision)"))
  (return 500.0 700.0))

(fn `SetMovementSpeed`
  (params (Speed :type "/Game/MyContent/Enemies/AI/Data/Enum/E_MovementSpeed Enum" :default "NewEnumerator0"))
  (returns (ReturnValue :type "Float (double-precision)"))
  (return (select `/Game/MyContent/Enemies/AI/Data/Enum/E_MovementSpeed` Speed :`NewEnumerator1` 150.0 :`NewEnumerator2` 250.0 :`NewEnumerator3` 400.0)))

(fn `TakeDamage`
  (params (DamageInfo :type "/Game/MyContent/BP/DamageSys/S_DamageInfo Structure") (`Damage Source` :type "Actor Object Reference"))
  (returns (WasDamage :type Boolean))
  (bind _wasdamage (`parent.TakeDamage` DamageInfo `Damage Source`))
  (if (`self.IsTeleport`)
    (`self.OnTeleportEnd`))
  (return _wasdamage))

(fn `UserConstructionScript`
  (`parent.UserConstructionScript`))