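; Mage enemy Blueprint that attacks from range with magic spells and can teleport, with its own movement speeds and ideal attack and defend ranges.
; Attack plays a cast montage whose Fire notify launches a damaging spell from the hand toward the target through BPCAttacks.
; Teleport is a disguised fast flight: AIMoveTo moves the hidden, pawn-ignoring mage with fireball effects, then TeleportEnd restores it, broadcasts completion and briefly delays re-use.
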(event `/Game/MyContent/Enemies/AI/BPI_EnemyAI.Attack`
  (params (AttackTarget :type "Actor Object Reference"))
  (bind _notifyname (`|PlayMontage` (`self.Mesh`) "/Game/MyContent/Anim/Magic/AM_Magic_Standing1HMagicAttack01_UE.AM_Magic_Standing1HMagicAttack01_UE")
    (:`OnCompleted`
      (`/Game/MyContent/Enemies/AI/BPI_EnemyAI.AttackEnd` AttackTarget :!label _label))
    (:`OnInterrupted`
      (goto _label))
    (:`OnNotifyBegin`
      (switch `name` _notifyname
        (:`Fire`
          (`/Game/MyContent/BP/Attack/BPC_Attacks.MagicSpell` (`self.BPC_Attacks`) (`KismetMathLibrary.MakeTransform` (`SceneComponent.GetSocketLocation` (`self.Mesh`) "hand_r_RifleSocket") (`KismetMathLibrary.FindLookAtRotation` (`self.K2_GetActorLocation`) (`self.K2_GetActorLocation` AttackTarget))) (make `/Game/MyContent/BP/DamageSys/S_DamageInfo` 30.0 "NewEnumerator2")))))))

(event `Teleport`
  (params (Location :type "Vector Structure"))
  (bind _charactermovement (`self.CharacterMovement`))
  (if (`self.IsTeleport`)
    (`KismetSystemLibrary.DelayUntilNextTick`)
    (`self.OnTeleportEnd`)
    (else
      (set `self.IsTeleport` true)
      (`CharacterMovementComponent.SetMovementMode` _charactermovement "MOVE_Flying" 0)
      (set `CharacterMovementComponent.MaxFlySpeed` 5000.0 _charactermovement)
      (set `CharacterMovementComponent.MaxAcceleration` 99999.0 _charactermovement)
      (`SceneComponent.SetVisibility` (`self.Mesh`) false true)
      (`PrimitiveComponent.SetCollisionResponseToChannel` (`self.CapsuleComponent`) "ECC_Pawn" "ECR_Ignore")
      (bind _returnvalue (`NiagaraFunctionLibrary.SpawnSystemAtLocation` "/Game/MyContent/Particle/NS_FireBallDead.NS_FireBallDead" (`SceneComponent.GetSocketLocation` (`self.Mesh`) "spine_01")))
      (set `self.TeleportBodyEffect` _returnvalue)
      (bind _returnvalue_2 (`NiagaraFunctionLibrary.SpawnSystemAttached` "/Game/MyContent/Particle/NS_FireBall.NS_FireBall" (`self.Mesh`) "spine_01" (0.0 0.0 0.0) (struct) "KeepRelativeOffset"))
      (set `self.TeleportTrailEffect` _returnvalue_2)
      (`self.StopAnimMontage` null)
      (`|AIMoveTo` self Location null 15.0
        (:`OnSuccess`
          _)
        (:`OnFail`
          _))
      (`self.TeleportEnd`))))

(event `TeleportEnd`
  (bind _charactermovement (`self.CharacterMovement`))
  (`MovementComponent.StopMovementImmediately` _charactermovement)
  (`CharacterMovementComponent.SetMovementMode` _charactermovement "MOVE_Walking" 0)
  (set `CharacterMovementComponent.MaxAcceleration` 1500.0 _charactermovement)
  (`SceneComponent.SetVisibility` (`self.Mesh`) true true)
  (`PrimitiveComponent.SetCollisionResponseToChannel` (`self.CapsuleComponent`) "ECC_Pawn" "ECR_Block")
  (`self.OnTeleportEnd`)
  (`KismetSystemLibrary.Delay` 0.5)
  (set `self.IsTeleport` false)
  (`|ExecutionSequence`
    (:`then_0`
      (bind _teleportbodyeffect (`self.TeleportBodyEffect`)
        (:`then`
          (`ActorComponent.K2_DestroyComponent` _teleportbodyeffect))
        (:`else`)))
    (:`then_1`
      (bind _teleporttraileffect (`self.TeleportTrailEffect`)
        (:`then`
          (`ActorComponent.K2_DestroyComponent` _teleporttraileffect))
        (:`else`)))))

(fn `GetIdealRange`
  (returns (AttackRadius :type "Float (double-precision)") (DefendRadius :type "Float (double-precision)"))
  (return 500.0 700.0))

(fn `SetMovementSpeed`
  (params (Speed :type "/Game/MyContent/Enemies/AI/Data/Enum/E_MovementSpeed Enum" :default "NewEnumerator0"))
  (returns (ReturnValue :type "Float (double-precision)"))
  (return (select `/Game/MyContent/Enemies/AI/Data/Enum/E_MovementSpeed` Speed :`NewEnumerator1` 150.0 :`NewEnumerator2` 250.0 :`NewEnumerator3` 400.0)))

(fn `UserConstructionScript`
  (`parent.UserConstructionScript`))