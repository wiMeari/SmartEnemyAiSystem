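; BP_AOE_Heal is a heal area-of-effect actor that adds a Niagara visual to its parent's Trigger behavior.
; On Trigger it calls the parent, spawns NS_Heal at its location and sets the effect's RingRadius from Radius.
; When the actor is destroyed, it deactivates the effect and binds to OnSystemFinished to destroy the component once the system finishes.
; No healing logic is defined in this Blueprint itself.
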(event `self.Trigger`
  (`parent.Trigger`)
  (bind _returnvalue (`NiagaraFunctionLibrary.SpawnSystemAtLocation` "/Game/MyContent/Particle/NS_Heal.NS_Heal" (`self.K2_GetActorLocation`)))
  (bind _output_get (set `self.NewVar` _returnvalue))
  (`NiagaraComponent.SetVariableFloat` _returnvalue "RingRadius" (`self.Radius`))
  (`NiagaraComponent.SetVariableFloat` _output_get "RingRadius" (`self.Radius`))
  (add `self.OnDestroyed` (delegate `OnDestroyed_事件`)))

(event `OnDestroyed_事件` :!signature `self.OnDestroyed`
  (params (DestroyedActor :type "Actor Object Reference"))
  (bind _newvar (`self.NewVar`)
    (:`then`
      (`ActorComponent.Deactivate` _newvar)
      (add `NiagaraComponent.OnSystemFinished` _newvar (delegate `OnSystemFinished_事件`)))
    (:`else`)))

(event `OnSystemFinished_事件`
  (params (PSystem :type "NiagaraComponent Object Reference"))
  (`ActorComponent.K2_DestroyComponent` PSystem))

(fn `UserConstructionScript`
  (`parent.UserConstructionScript`))