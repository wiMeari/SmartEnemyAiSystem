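; Attack component that gives its owner a fireball spell and a hitscan bullet attack.
; MagicSpell spawns BP_FireBall ignoring the owner and binds its impact, which applies the spell's DamageInfo and fires OnAttackEnd.
; FireBullet line-traces for Pawns with debug drawing and damages the hit actor, without signalling attack end.
; Both attacks deal damage through TakeDamageMessage and report it to AI damage sensing with the owner as instigator.
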(event `MagicSpell`
  (params (SpawnTransform :type "Transform Structure") (DamageInfo :type "/Game/MyContent/BP/DamageSys/S_DamageInfo Structure"))
  (bind _returnvalue (`|SpawnActorFromClass` "/Game/MyContent/BP/Projectile/BP_FireBall.BP_FireBall_C" SpawnTransform "Undefined" "MultiplyWithRoot" (`self.GetOwner`) 1000.0 1000.0 0.0 null))
  (add `/Game/MyContent/BP/Projectile/BP_ProjectileBase.OnProjectileImpact` _returnvalue (delegate `OnProjectileImpact`))
  (`PrimitiveComponent.IgnoreActorWhenMoving` (`/Game/MyContent/BP/Projectile/BP_ProjectileBase.Sphere` _returnvalue) (`self.GetOwner`) true))

(event `OnProjectileImpact`
  (params (OtherActor :type "Actor Object Reference") (Hit :type "HitResult Structure"))
  (message `/Game/MyContent/BP/DamageSys/BPI_Damageable.TakeDamage` OtherActor (stale `MagicSpell` DamageInfo))
  (`AISense_Damage.ReportDamageEvent` OtherActor (`self.GetOwner`) (`.Amount_2_4911AAF8403F46AE6949C98284F04AC6` (break `/Game/MyContent/BP/DamageSys/S_DamageInfo` (stale `MagicSpell` DamageInfo))) (`Actor.K2_GetActorLocation` (`self.GetOwner`)))
  (`self.OnAttackEnd`))

(event `FireBullet`
  (params (TraceStart :type "Vector Structure") (TraceEnd :type "Vector Structure") (DamageInfo :type "/Game/MyContent/BP/DamageSys/S_DamageInfo Structure"))
  (bind (_outhit _returnvalue) (`KismetSystemLibrary.LineTraceSingleForObjects` :`Start` TraceStart :`End` TraceEnd :`ObjectTypes` (`|MakeArray` "ObjectTypeQuery3" :!type "EObjectTypeQuery Enum") :`DrawDebugType` "ForDuration"))
  (if _returnvalue
    (bind (_bblockinghit _binitialoverlap _time _distance _location _impactpoint _normal _impactnormal _physmat _hitactor) (`GameplayStatics.BreakHitResult` _outhit))
    (message `/Game/MyContent/BP/DamageSys/BPI_Damageable.TakeDamage` _hitactor DamageInfo)
    (`AISense_Damage.ReportDamageEvent` _hitactor (`self.GetOwner`) (`.Amount_2_4911AAF8403F46AE6949C98284F04AC6` (break `/Game/MyContent/BP/DamageSys/S_DamageInfo` DamageInfo)) (`Actor.K2_GetActorLocation` (`self.GetOwner`)))))