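; BP_ProjectileBase is a base projectile actor with a Sphere collision component and projectile movement.
; The construction script copies its initial speed, maximum speed and gravity variables into ProjectileMovement.
; Logic to broadcast OnProjectileImpact with the hit result, ignoring the owner, exists but is disconnected, so the sphere's hit event currently does nothing.
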(event `self.ReceiveTick`
  (params (DeltaSeconds :type "Float (single-precision)")))

(event `self.Sphere.OnComponentHit`
  (params (HitComponent :type "PrimitiveComponent Object Reference") (OtherActor :type "Actor Object Reference") (OtherComp :type "PrimitiveComponent Object Reference") (NormalImpulse :type "Vector Structure") (Hit :type "HitResult Structure (by ref)")))

(fn `UserConstructionScript`
  (bind _projectilemovement (`self.ProjectileMovement`))
  (set `ProjectileMovementComponent.InitialSpeed` (`self.初始速度`) _projectilemovement)
  (set `ProjectileMovementComponent.MaxSpeed` (`self.最大速度`) _projectilemovement)
  (set `ProjectileMovementComponent.ProjectileGravityScale` (`self.重力`) _projectilemovement))