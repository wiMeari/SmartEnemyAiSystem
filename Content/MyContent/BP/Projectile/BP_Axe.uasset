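; BP_Axe is an axe projectile Blueprint that adds a continuous spinning motion on top of its parent class.
; After the parent BeginPlay, SpinAxe plays the Rotation timeline, which drives the world pitch of RotationPoint while taking roll and yaw from StaticMesh1.
; The spin loops by calling SpinAxe again whenever the timeline finishes, so Tick is not used.
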(event `self.ReceiveBeginPlay`
  (`parent.ReceiveBeginPlay`)
  (`self.SpinAxe`))

(event `SpinAxe`
  (bind (_returnvalue_roll _returnvalue_pitch _returnvalue_yaw) (`KismetMathLibrary.BreakRotator` (`SceneComponent.K2_GetComponentRotation` (`self.StaticMesh1`))))
  (bind (_direction _zrotation) (`Timeline|Rotation` :!via `PlayFromStart`)
    (:`Update`
      (`SceneComponent.K2_SetWorldRotation` (`self.RotationPoint`) (`KismetMathLibrary.MakeRotator` _returnvalue_roll _zrotation _returnvalue_yaw) false false))
    (:`Finished`
      (`self.SpinAxe`))))

(fn `UserConstructionScript`
  (`parent.UserConstructionScript`))