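; BP_FireBall2 is a fireball projectile with a collision sphere and a Niagara fireball effect.
; On hit, it broadcasts OnProjectileImpact with the hit actor and result, then spawns the NS_FireBallDead effect at the hit location.
; It disables sphere collision and deactivates the fireball effect, destroying itself when that system finishes.
; A binding to clean up the spawned impact effect exists but never runs.
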(event `self.ReceiveTick`
  (params (DeltaSeconds :type "Float (single-precision)")))

(event `self.Sphere.OnComponentHit`
  (params (HitComponent :type "PrimitiveComponent Object Reference") (OtherActor :type "Actor Object Reference") (OtherComp :type "PrimitiveComponent Object Reference") (NormalImpulse :type "Vector Structure") (Hit :type "HitResult Structure (by ref)"))
  (bind _ns_fireball (`self.NS_FireBall`))
  (`self.OnProjectileImpact` OtherActor Hit)
  (bind _returnvalue (`NiagaraFunctionLibrary.SpawnSystemAtLocation` "/Game/MyContent/Particle/NS_FireBallDead.NS_FireBallDead" (`.Location` (`GameplayStatics.BreakHitResult` Hit))))
  (bind _output_get (set `self.NewVar` _returnvalue))
  (`PrimitiveComponent.SetCollisionEnabled` (`self.Sphere`) "NoCollision")
  (`ActorComponent.Deactivate` _ns_fireball)
  (add `NiagaraComponent.OnSystemFinished` _ns_fireball (delegate `OnSystemFinished_事件`)))

(event `OnSystemFinished_事件`
  (params (PSystem :type "NiagaraComponent Object Reference"))
  (`self.K2_DestroyActor`))

(event `OnSystemFinished_事件_0`
  (params (PSystem :type "NiagaraComponent Object Reference"))
  (`ActorComponent.K2_DestroyComponent` PSystem))

(fn `UserConstructionScript`)